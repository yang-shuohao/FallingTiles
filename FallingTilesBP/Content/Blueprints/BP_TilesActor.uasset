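; One falling row in a Piano Tiles-style game, with four touchable sprite keys, one active, optionally as a start button.
; Initialization colors keys and snaps it above the previous row; Tick moves it down at the owner's fall speed.
; Correct in-order taps mark it selected, request the next tile and self-destroy after a delay.
; Wrong-key taps flash red and report game over; game state and speed come via owner messages.
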(event OnInputTouchBegin(Key01_Sprite)
  (params (FingerIndex :type ETouchIndex%20Enum :default "Touch1") (TouchedComponent :type Primitive%20Component%20Object%20Reference))
  ;[1 0.3222 0.8165] 选择触发事件
  (CallFunction|SelectTile 0 TouchedComponent))

(event OnInputTouchBegin(Key02_Sprite)
  (params (FingerIndex :type ETouchIndex%20Enum :default "Touch1") (TouchedComponent :type Primitive%20Component%20Object%20Reference))
  ;[1 0.3222 0.8165] 选择触发事件
  (CallFunction|SelectTile 1 TouchedComponent))

(event OnInputTouchBegin(Key03_Sprite)
  (params (FingerIndex :type ETouchIndex%20Enum :default "Touch1") (TouchedComponent :type Primitive%20Component%20Object%20Reference))
  ;[1 0.3222 0.8165] 选择触发事件
  (CallFunction|SelectTile 2 TouchedComponent))

(event OnInputTouchBegin(Key04_Sprite)
  (params (FingerIndex :type ETouchIndex%20Enum :default "Touch1") (TouchedComponent :type Primitive%20Component%20Object%20Reference))
  ;[1 0.3222 0.8165] 选择触发事件
  (CallFunction|SelectTile 3 TouchedComponent))

(event Custom|Initilize%20Tiles
  (params (IsStartButton :type Boolean) (PreviousTile :type BP%20Tiles%20Actor%20Object%20Reference) (ActiveKeyIndex :type Integer) (LocationZ :type Float%20%28double-precision%29))
  ;[0.04957 0.3083 1] 初始化Tiles
  (Variables|Default|SetIsStartButton IsStartButton)
  (Variables|Default|SetPreviousTile PreviousTile)
  (Variables|Default|SetActiveKeyIndex ActiveKeyIndex)
  (Transformation|SetActorLocation (Math|Vector|MakeVector 0.0 0.0 LocationZ) false false)
  (Utilities|FlowControl|Sequence
    (:then_0
      (Variables|Default|SetIsSelected false)
      (for (_array_element _array_index) (Utilities|Array|MakeArray (Variables|Default|GetKey01_Sprite) (Variables|Default|GetKey02_Sprite) (Variables|Default|GetKey03_Sprite) (Variables|Default|GetKey04_Sprite))
        (Sprite|SetSpriteColor _array_element (select (== _array_index (Variables|Default|GetActiveKeyIndex)) (select (Variables|Default|GetIsStartButton) "(R=1.000000,G=1.000000,B=1.000000,A=1.000000)" "(R=0.000000,G=0.000000,B=0.000000,A=1.000000)") "(R=1.000000,G=1.000000,B=1.000000,A=0.000000)"))
        (Rendering|Components|Sprite|SetSprite _array_element (select (Variables|Default|GetIsStartButton) "/Game/Assets/Sprites/T_StartTile_Sprite.T_StartTile_Sprite" "/Game/Assets/Sprites/T_Tile_Sprite.T_Tile_Sprite"))))
    (:then_1
      (if (not (Variables|Default|GetIsStartButton))
        (if (Utilities|Operators|NotEqual(!=) (Transformation|GetActorLocation (Variables|Default|GetPreviousTile)) (- (Transformation|GetActorLocation) "0,0,175.000000") 0.25)
          (Transformation|SetActorLocation (+ (Transformation|GetActorLocation (Variables|Default|GetPreviousTile)) "0,0,175.000000") false false))))))

(event Custom|XXXXX
  ;[0.5852 0.4316 1] 游戏结束处理
  (Variables|Default|SetSpriteComponent (Utilities|Array|Get(acopy) (Utilities|Array|MakeArray (Variables|Default|GetKey01_Sprite) (Variables|Default|GetKey02_Sprite) (Variables|Default|GetKey03_Sprite) (Variables|Default|GetKey04_Sprite)) (Variables|Default|GetActiveKeyIndex)))
  (Sprite|SetSpriteColor (stale Custom|GameOver _output_get) (Variables|Default|GetErrorColor))
  (Rendering|Components|Sprite|SetSprite (Variables|Default|GetSpriteComponent) "/Game/Assets/Sprites/T_TileTransparent_Sprite.T_TileTransparent_Sprite")
  (Timeline|FlashingTimeline PlayFromStart
    (:Finished
      (Rendering|SetVisibility (Variables|Default|GetSpriteComponent) true false))
    (:Toggle%20Visibility
      (Rendering|ToggleVisibility (Variables|Default|GetSpriteComponent) false))))

(event Custom|GameOver
  (params (Object :type Primitive%20Component%20Object%20Reference))
  ;[0.5852 0.4316 1] 游戏结束处理
  (Class|BPInterface|GameOver(Message) (Components|GetOwner))
  (bind _aspaper_sprite_component (Utilities|Casting|CastToPaperSpriteComponent Object))
  (bind _output_get (Variables|Default|SetSpriteComponent _aspaper_sprite_component))
  (Sprite|SetSpriteColor _output_get (Variables|Default|GetErrorColor))
  (Rendering|Components|Sprite|SetSprite (Variables|Default|GetSpriteComponent) "/Game/Assets/Sprites/T_TileTransparent_Sprite.T_TileTransparent_Sprite")
  (Timeline|FlashingTimeline PlayFromStart
    (:Finished
      (Rendering|SetVisibility (Variables|Default|GetSpriteComponent) true false))
    (:Toggle%20Visibility
      (Rendering|ToggleVisibility (Variables|Default|GetSpriteComponent) false))))

(event Custom|Collect
  (params (Object :type Primitive%20Component%20Object%20Reference))
  ;[1 0.852 0.3517] 正确选择，改为绿色
  (Variables|Default|SetIsSelected true)
  (Class|BPInterface|SpawnNextTile(Message) (Components|GetOwner) false)
  (bind _aspaper_sprite_component (Utilities|Casting|CastToPaperSpriteComponent Object))
  (Sprite|SetSpriteColor _aspaper_sprite_component (Variables|Default|GetCheckColor))
  (Rendering|Components|Sprite|SetSprite _aspaper_sprite_component "/Game/Assets/Sprites/T_TileTransparent_Sprite.T_TileTransparent_Sprite")
  (CallFunction|Destroy))

(event Custom|SelectTile
  (params (InputPin :type Integer) (InputPin2 :type Primitive%20Component%20Object%20Reference))
  ;[1 0.2783 0.2384] 选择Tiles
  (bind _returnvalue (Class|BPInterface|GetGameStatus(Message) (Components|GetOwner)))
  (switch Utilities|FlowControl|Switch|SwitchonEnum_GameStatus _returnvalue
    (:NewEnumerator0
      (if (and (== (Variables|Default|GetActiveKeyIndex) InputPin) (Variables|Default|GetIsStartButton))
        (Class|BPInterface|StartNewGame(Message) (Components|GetOwner))
        (CallFunction|Collect InputPin2)))
    (:NewEnumerator1
      (if (== (Variables|Default|GetActiveKeyIndex) InputPin)
        (bind _previoustile (Variables|Default|GetPreviousTile)
          (:then
            (if (Variables|BP_TilesActor_C|GetIsSelected _previoustile)
              (CallFunction|Collect InputPin2 :!label _label)
              (Audio|PlaySound2D "/Game/Sounds/pinkyfinger__piano-c.pinkyfinger__piano-c" 1.0 1.0 0.0 0 0)))
          (:else
            (goto _label)))
        (else
          (CallFunction|GameOver InputPin2))))))

(event Custom|Destroy
  ;[0 1 0.7805] 4秒以后销毁
  (Utilities|FlowControl|Delay 4.0)
  (Actor|DestroyActor))

(event EventTick
  (params (DeltaSeconds :type Float%20%28single-precision%29))
  ;[0.1875 1 1] 不断更新Z轴位置，向下移动
  (bind _returnvalue (Class|BPInterface|GetFallSpeed(Message) (Components|GetOwner)))
  (Transformation|AddActorWorldOffset (* "0,0,-1.000000" (* _returnvalue DeltaSeconds))))

(fn ConstructionScript)