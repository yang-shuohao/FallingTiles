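; Game manager for a falling piano-tiles game, owning game status, fall speed, score UI and music.
; It seeds seven stacked BP_TilesActor rows, the first a start button, chaining each to the previous with a non-repeating random key.
; During play, speed ramps to a cap and each spawn scores and starts a one-second game-over timer.
; Music volume follows that timer's remaining time, while pitch periodically updates from fall speed.
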(event Custom|OnGameOver
  ;[0.4301 1 0.7076] 生成下一个Tile
  (CallFunction|GameOver)
  (bind _outactors (Actor|GetAllActorsOfClass "/Game/Blueprints/BP_TilesActor.BP_TilesActor_C"))
  (Default|XXXXX _outactors))

(event Custom|UpdateMusicPitchMuliplier
  ;[1 0.4366 0.9654] 开始新游戏
  (bind _gamemusic (Variables|Default|GetGameMusic)
    (:then
      (Audio|Components|Audio|SetPitchMultiplier _gamemusic (+ (Math|Float|Power (- (/ (Variables|Default|GetFallSpeed) 4.5e+02) 1.0) 1e+01) 1.0)))
    (:else)))

(event EventBeginPlay
  (bind _returnvalue (Viewport|GetViewportSize))
  ;[0 0.2706 1] 创建分数UI，生成7个Tiles
  (bind _returnvalue_2 (UserInterface|CreateWidget "/Game/Blueprints/Widgets/WG_GameScore.WG_GameScore_C" (Game|GetPlayerController 0)))
  (bind _output_get (Variables|Default|SetWGGameScore _returnvalue_2))
  (UserInterface|Viewport|AddtoViewport _output_get 0)
  (CallFunction|SetFallSpeed 0.0)
  (Variables|Default|SetNextTileLocationZ (+ (/ (Variables|Default|GetTileHeight) 2.0) (* (/ (.y _returnvalue) (.x _returnvalue)) 2e+02 -1.0)))
  (for _index (range 0 6)
    (CallFunction|SpawnNextTile (== _index 0))))

(event EventSpawnNextTile
  (params (IsStartButton :type Boolean))
  (bind _score (Variables|Default|GetScore))
  ;[0.4301 1 0.7076] 生成下一个Tile
  (Variables|Default|SetLastSpawnPoint (CallFunction|GetNextSpawnPointIndex (Variables|Default|GetLastSpawnPoint)))
  (bind _returnvalue (Game|SpawnActorfromClass "/Game/Blueprints/BP_TilesActor.BP_TilesActor_C" (Math|Conversions|ToTransform(Vector) (Math|Vector|MakeVector 0.0 0.0 (Variables|Default|GetNextTileLocationZ))) "AlwaysSpawn" self 0))
  (Default|InitilizeTiles _returnvalue IsStartButton (Variables|Default|GetLastSpawnedTile) (Variables|Default|GetLastSpawnPoint) (Variables|Default|GetNextTileLocationZ))
  (Variables|Default|SetLastSpawnedTile _returnvalue)
  (Variables|Default|SetNextTileLocationZ (+ (Variables|Default|GetNextTileLocationZ) (Variables|Default|GetTileHeight)))
  (if (Utilities|Enum|Equal(Enum) (Variables|Default|GetGameStatus) "NewEnumerator1")
    (Math|Integer|IncrementInt _score
      (:%20%20
        (Default|UpdateScoreText (Variables|Default|GetWGGameScore) _score)
        (bind _returnvalue_2 (Utilities|Time|SetTimerbyEvent (delegate Custom|OnGameOver) 1.0))
        (Variables|Default|SetTimerHandle _returnvalue_2)))))

(event EventGameOver
  ;[1 0.3591 0.2993] 游戏结束
  (if (Utilities|Enum|Equal(Enum) (Variables|Default|GetGameStatus) "NewEnumerator1")
    (Utilities|Time|ClearandInvalidateTimerbyHandle (Variables|Default|GetTimerHandle))
    (Audio|Components|Audio|Stop (Variables|Default|GetGameMusic))
    (Audio|PlaySound2D "/Game/Sounds/Mission_failed_Defeat_Try_Again_Sound_Effects_SFX__2.Mission_failed_Defeat_Try_Again_Sound_Effects_SFX__2" 1.0 1.0 0.0 0 0)
    (CallFunction|SetGameStatus "NewEnumerator2")
    (Utilities|FlowControl|Delay 2.0)
    (bind _returnvalue (UserInterface|CreateWidget "/Game/Blueprints/Widgets/WG_GameOver.WG_GameOver_C"))
    (UserInterface|Viewport|AddtoViewport _returnvalue 0)))

(event EventTick
  (params (DeltaSeconds :type Float%20%28single-precision%29))
  (bind _timerhandle (Variables|Default|GetTimerHandle))
  ;[1 0.1506 0.9505] 播放背景音效，下落速度不断增加
  (Variables|Default|SetDeltaSecond DeltaSeconds)
  (switch Utilities|FlowControl|Switch|SwitchonEnum_GameStatus (Variables|Default|GetGameStatus)
    (:NewEnumerator1
      (Variables|Default|SetFallSpeed (Math|Float|Clamp(Float) (+ (Variables|Default|GetFallSpeed) (* (Variables|Default|GetDeltaSecond) 15.0)) 0.0 (Variables|Default|GetMaxFallSpeed)))
      (Audio|Components|Audio|SetVolumeMultiplier (Variables|Default|GetGameMusic) (select (Utilities|Time|IsTimerActivebyHandle _timerhandle) (Math|Float|Lerp 0.0 1.0 (Utilities|Time|GetTimerRemainingTimebyHandle _timerhandle)) 1.0) :!class /Script/Engine.AudioComponent))
    (:NewEnumerator2
      (Variables|Default|SetFallSpeed 0.0))))

(event EventSetFallSpeed
  (params (Value :type Float%20%28double-precision%29))
  ;[1 0.7284 0.8754] 下落速度
  (Variables|Default|SetFallSpeed Value))

(event EventSetGameStatus
  (params (Value :type Enum_GameStatus%20Enum :default "NewEnumerator0"))
  ;[0.4163 0.6612 1] 游戏状态
  (Variables|Default|SetGameStatus Value))

(event EventStartNewGame
  ;[1 0.4366 0.9654] 开始新游戏
  (CallFunction|SetFallSpeed 4e+02)
  (CallFunction|SetGameStatus "NewEnumerator1")
  (bind _returnvalue (Audio|SpawnSound2D "/Game/Sounds/gem_popper.gem_popper" 1.0 1.0 0.0 0))
  (Variables|Default|SetGameMusic _returnvalue)
  (CallFunction|UpdateMusicPitchMuliplier)
  (Utilities|Time|SetTimerbyEvent (delegate Custom|UpdateMusicPitchMuliplier) 1.0 true))

(fn ConstructionScript)

(fn GetNextSpawnPointIndex
  (params (LastIndex :type Integer))
  (bind _output_get (LocalVariables|SetIndicesArrayLocal (Utilities|Array|MakeArray 0 1 2 3)))
  (Utilities|Array|RemoveIndex _output_get LastIndex)
  (Utilities|Array|Shuffle (LocalVariables|GetIndicesArrayLocal))
  (return (Utilities|Array|Get(acopy) (LocalVariables|GetIndicesArrayLocal))))

(fn GetFallSpeed
  (return (Variables|Default|GetFallSpeed)))

(fn GetGameStatus
  (return (Variables|Default|GetGameStatus)))